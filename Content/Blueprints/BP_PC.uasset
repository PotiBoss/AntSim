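; BP_PC is a player controller that handles pheromone display toggling and food inspection.
; The E key calls SwitchPheromoneVisibilty, which is defined outside this graph.
; A left click, when no FoodWidget is valid, traces under the cursor and, on hitting a Food actor, creates a WBP_Food widget, binds that actor and initializes it.
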(event EventBeginPlay)

(event EventTick
  (params (DeltaSeconds :type Float%20%28single-precision%29)))

(event Input|MouseEvents|LeftMouseButton
  (params (Key :type Key%20Structure :default "None"))
  (:Pressed
    (if (not (Utilities|IsValid (Variables|Default|GetFoodWidget)))
      (bind _asfood (Utilities|Casting|CastToFood (.hitactor (.HitResult (Game|Player|GetHitResultUnderCursorbyChannel "TraceTypeQuery1" true)))))
      (bind _returnvalue (UserInterface|CreateWidget "/Game/Blueprints/WBP_Food.WBP_Food_C"))
      (bind _output_get (Variables|Default|SetFoodWidget _returnvalue))
      (UserInterface|Viewport|AddtoViewport _output_get 0)
      (Variables|/Script/AntSim.FoodWidget|SetFood _output_get _asfood)
      (Class|FoodWidget|Init _output_get))))

(event Input|KeyboardEvents|E
  (params (Key :type Key%20Structure :default "None"))
  (:Pressed
    (Class|PC|SwitchPheromoneVisibilty)))

(fn ConstructionScript)